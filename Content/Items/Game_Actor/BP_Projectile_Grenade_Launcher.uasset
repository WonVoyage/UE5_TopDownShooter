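; Grenade launcher projectile actor that deals area damage when it receives damage itself.
; Its AnyDamage event runs a sequence that applies radial damage with falloff, then a second plain radial damage, both centered on the BulletMesh location.
; A debug sphere is drawn at the same point after the second hit.
; BeginPlay, overlap and Tick are disabled stubs, and the construction script only calls the parent.
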(event `self.ReceiveAnyDamage`
  (params (Damage :type "Float (single-precision)") (DamageType :type "DamageType Object Reference") (InstigatedBy :type "Controller Object Reference") (DamageCauser :type "Actor Object Reference"))
  (bind _returnvalue (`SceneComponent.K2_GetComponentLocation` (`self.Bullet_Mesh`)))
  (`|ExecutionSequence`
    (:`then_0`
      (`GameplayStatics.ApplyRadialDamageWithFalloff` :`Origin` _returnvalue :`DamageCauser` null :`InstigatedByController` null))
    (:`then_1`
      (`GameplayStatics.ApplyRadialDamage` :`Origin` _returnvalue :`DamageCauser` null :`InstigatedByController` null)
      (`KismetSystemLibrary.DrawDebugSphere` _returnvalue))))

(fn `UserConstructionScript`
  (`parent.UserConstructionScript`))