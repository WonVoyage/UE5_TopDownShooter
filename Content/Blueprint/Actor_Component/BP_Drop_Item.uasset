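; BP_Drop_Item is an actor component that drops an ammo pickup at its owner's location.
; Its Drop event takes a weapon type, sets the ammo count for it, then spawns a Pickup_Ammo with that type and count.
; It then assigns the pickup a type-specific mesh and enlarges it.
; Only Rifle and Grenade Launcher have counts and meshes defined.
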(event `Drop`
  (params (Type :type "EWeapon_Type Enum" :default "Pistol"))
  (set `self.Type` Type)
  (`|ExecutionSequence`
    (:`then_0`
      (switch `EWeapon_Type` (`self.Type`)
        (:`Rifle`
          (set `self.Count` 15))
        (:`Grenade_Launcher`
          (set `self.Count` 2))))
    (:`then_1`
      (bind _returnvalue (`|SpawnActorFromClass` "/Game/Blueprint/Interaction_Environment/Pickup_Ammo.Pickup_Ammo_C" (`KismetMathLibrary.MakeTransform` (`Actor.K2_GetActorLocation` (`self.GetOwner`))) "AlwaysSpawn" "MultiplyWithRoot" null (`self.Type`) (`self.Count`) null))
      (bind _staticmesh (`/Game/Blueprint/Interaction_Environment/Pickup.StaticMesh` _returnvalue))
      (`StaticMeshComponent.SetStaticMesh` _staticmesh (select `EWeapon_Type` (`self.Type`) :`Rifle` "/Game/MilitaryWeapSilver/Pickups/AssaultRifle_Pickup.AssaultRifle_Pickup" :`Grenade_Launcher` "/Game/MilitaryWeapSilver/Pickups/GrenadeLauncher_Pickup.GrenadeLauncher_Pickup" :!type "StaticMesh Object Reference"))
      (`SceneComponent.SetRelativeScale3D` _staticmesh (3.0 3.0 3.0)))))