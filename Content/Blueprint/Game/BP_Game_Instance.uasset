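; Game instance Blueprint that handles hosting and joining multiplayer game sessions.
; Creating a session stores the player limit, takes a LAN option and opens Lobby_Level on success.
; Joining uses a supplied search result with no explicit success logic, and both failure paths only print a placeholder "Hello".
; CreateSession and JoinSession events forward their arguments to game-session create and join calls.
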(event `Create_Game_Sesion`
  (params (Max_Players :type Integer) (bUseLAN :type Boolean))
  (bind _output_get (set `self.Max_Players` Max_Players))
  (`CreateSessionCallbackProxy.CreateSession` (`GameplayStatics.GetPlayerController` 0) _output_get bUseLAN
    (:`OnSuccess`
      (`GameplayStatics.OpenLevel` "Lobby_Level" true "Listen"))
    (:`OnFailure`
      (`KismetSystemLibrary.PrintString` "Hello"))))

(event `Join_Game_Session`
  (params (SearchResult :type "BlueprintSessionResult Structure (by ref)"))
  (`JoinSessionCallbackProxy.JoinSession` (`GameplayStatics.GetPlayerController` 0) SearchResult
    (:`OnFailure`
      (`KismetSystemLibrary.PrintString` "Hello"))))

(event `/Game/Blueprint/Game/Lobby/BPI_Network.Join_Session`
  (params (Session_To_Join :type "BlueprintSessionResult Structure"))
  (`self.Join_Game_Session` Session_To_Join))

(event `/Game/Blueprint/Game/Lobby/BPI_Network.Create_Session`
  (params (Max_Players :type Integer) (`Use LAN` :type Boolean))
  (`self.Create_Game_Sesion` Max_Players `Use LAN`))