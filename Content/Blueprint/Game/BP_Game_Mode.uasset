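; Game mode that handles player death, lives, checkpoint respawns and the score-based end of the game.
; On death it drops the current weapon, unpossesses and expires the pawn, then either shows the end-game widget or respawns at hard-coded checkpoint 2.
; RespawnCharacter maps a checkpoint enum to named player starts.
; Enemy kills add score, and reaching the threshold unpossesses the player and shows the same end-game widget.
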(event `self.BP_Dead`
  (bind _asbp_top_down_character (cast `/Game/Blueprint/Character/BP_TopDownCharacter` (`GameplayStatics.GetPlayerPawn` 0))
    (:`then`
      (bind _returnvalue (`Inventory.Get_Weapon_Name_By_Slot_Index` (`TDSCharacter.Inventory` _asbp_top_down_character) (`TDSCharacter.Curr_Slot_Index` _asbp_top_down_character)))
      (`/Game/Blueprint/Character/BP_TopDownCharacter.Drop_Item` :`self` _asbp_top_down_character :`Item` (make `Drop_Item` null null (make `Weapon_Slot` _returnvalue (`TDSCharacter.Weapon_Info` _asbp_top_down_character))))
      (`Controller.UnPossess` (`GameplayStatics.GetPlayerController` 0))
      (`self.SetLifeSpan` _asbp_top_down_character 3.0)
      (bind _result (`/Engine/EditorBlueprintResources/StandardMacros.DecrementInt` (`self.Lives`))
        (:`  `
          (if (< _result 0)
            (bind _returnvalue_2 (`|CreateWidget` "/Game/Blueprint/Widget/BPW_End_Game.BPW_End_Game_C"))
            (`UserWidget.AddToViewport` _returnvalue_2 0)
            (else
              (`self.Respawn Character` "NewEnumerator1")
              (bind _asbp_top_down_character_2 (cast `/Game/Blueprint/Character/BP_TopDownCharacter` (`GameplayStatics.GetPlayerPawn` 0))
                (:`then`
                  (`Health.Change_Health` (`TDSCharacter.Health` _asbp_top_down_character_2) -999.0)
                  (set `TDSCharacter.Is_Alive` true _asbp_top_down_character_2))
                (:`CastFailed`
                  (`KismetSystemLibrary.PrintString` "Can't cast in BPW_END_GAME_WITH_CHECKPOINT" true true (struct :`G` 0.66 :`B` 1.0 :`A` 1.0) 10.0))))))))
    (:`CastFailed`
      (`KismetSystemLibrary.PrintString` "Hello"))))

(fn `Enemy_Dead`
  (params (Score :type Integer))
  (`self.Increment_Score` Score))

(fn `Increment_Score`
  (params (Value :type Integer))
  (bind _output_get (set `self.Score` (+ (`self.Score`) Value)))
  (if (>= _output_get 15)
    (`Controller.UnPossess` (`GameplayStatics.GetPlayerController` 0))
    (bind _returnvalue (`|CreateWidget` "/Game/Blueprint/Widget/BPW_End_Game.BPW_End_Game_C"))
    (`UserWidget.AddToViewport` _returnvalue 0)))

(fn `Respawn Character`
  (params (Checkpoint :type "/Game/Blueprint/Checkpoints/E_Checkpoints Enum" :default "NewEnumerator0"))
  (`self.RestartPlayerAtPlayerStart` (`GameplayStatics.GetPlayerController` 0) (`self.K2_FindPlayerStart` null (select `/Game/Blueprint/Checkpoints/E_Checkpoints` Checkpoint :`NewEnumerator0` "Check_Point_1" :`NewEnumerator1` "Check_Point_2" :`NewEnumerator2` "Check_Point_3" :`NewEnumerator3` "Check_Point_4" :`NewEnumerator4` "Check_Point_5"))))

(fn `UserConstructionScript`)