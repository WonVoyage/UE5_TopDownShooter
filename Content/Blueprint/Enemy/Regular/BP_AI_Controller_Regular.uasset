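; AI controller for regular enemies that runs BT_Regular and starts it in the patrol chase state.
; AI Perception updates route hearing to Finding, successful non-hearing senses to Chasing, and lost senses to Patroling.
; These functions write the target object, last heard position, seen/heard flags and Chase_State to the blackboard for the tree.
; Finding and Chasing also draw debug spheres at the target's location.
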(event `self.ReceiveBeginPlay`
  (`self.RunBehaviorTree` "/Game/Blueprint/Enemy/Regular/AI/BT_Regular.BT_Regular")
  (`BlackboardComponent.SetValueAsEnum` (`AIBlueprintHelperLibrary.GetBlackboard` null) "Chase_State" 3))

(event `self.AI_Perception.OnTargetPerceptionUpdated`
  (params (Actor :type "Actor Object Reference") (Stimulus :type "AIStimulus Structure"))
  (set `self.Current_Target` Actor)
  (bind _returnvalue (`AIPerceptionSystem.GetSenseClassForStimulus` Stimulus))
  (if (== _returnvalue "/Script/AIModule.AISense_Hearing")
    (`self.Finding`)
    (elif (`.bSuccessfullySensed` (break `AIStimulus` Stimulus))
      (`self.Chasing`)
      (else
        (`self.Patroling`)))))

(fn `Chasing`
  (bind _returnvalue (`self.K2_GetActorLocation` (`self.Current_Target`)))
  (`BlackboardComponent.SetValueAsObject` (`AIBlueprintHelperLibrary.GetBlackboard` null) "Target_Object" (`self.Current_Target`))
  (`BlackboardComponent.SetValueAsBool` (`AIBlueprintHelperLibrary.GetBlackboard` null) "Target_Was_Seen" true)
  (`BlackboardComponent.SetValueAsBool` (`AIBlueprintHelperLibrary.GetBlackboard` null) "Target_Was_Heard" true)
  (`BlackboardComponent.SetValueAsEnum` (`AIBlueprintHelperLibrary.GetBlackboard` null) "Chase_State" 0)
  (`KismetSystemLibrary.DrawDebugSphere` _returnvalue 12.0 12 (struct :`R` 0.221679 :`G` 1.0 :`A` 1.0) 10.0)
  (`KismetSystemLibrary.DrawDebugString` _returnvalue "lost target here" null (struct :`A` 1.0) 10.0))

(fn `Finding`
  (`BlackboardComponent.SetValueAsVector` (`AIBlueprintHelperLibrary.GetBlackboard` null) "Target_Last_Position" (`self.K2_GetActorLocation` (`self.Current_Target`)))
  (`BlackboardComponent.SetValueAsBool` (`AIBlueprintHelperLibrary.GetBlackboard` null) "Target_Was_Heard" true)
  (`BlackboardComponent.SetValueAsEnum` (`AIBlueprintHelperLibrary.GetBlackboard` null) "Chase_State" 1)
  (`KismetSystemLibrary.DrawDebugSphere` (`self.K2_GetActorLocation` (`self.Current_Target`)) 12.0 12 (struct :`R` 1.0 :`G` 0.908667 :`A` 1.0) 10.0))

(fn `Patroling`
  (`/Engine/EditorBlueprintResources/StandardMacros.IsValid` (`self.Current_Target`)
    (:`Is Valid`
      (`BlackboardComponent.SetValueAsVector` (`AIBlueprintHelperLibrary.GetBlackboard` null) "Target_Position" (0.0 0.0 0.0))
      (`BlackboardComponent.SetValueAsObject` (`AIBlueprintHelperLibrary.GetBlackboard` null) "Target_Object" null)
      (`BlackboardComponent.SetValueAsBool` (`AIBlueprintHelperLibrary.GetBlackboard` null) "Target_Was_Seen" false)
      (`BlackboardComponent.SetValueAsBool` (`AIBlueprintHelperLibrary.GetBlackboard` null) "Target_Was_Heard" false)
      (`BlackboardComponent.SetValueAsEnum` (`AIBlueprintHelperLibrary.GetBlackboard` null) "Chase_State" 3))))

(fn `UserConstructionScript`)