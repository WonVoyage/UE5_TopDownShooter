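; Base enemy Blueprint that chases the first top-down player character found, re-issuing a move order every tick while it can move.
; Damage feeds a Health component, whose change event spawns a jittered damage display and randomly triggers a timed scream-montage stun that halts movement.
; On death it disables movement and attack, drops an optional pistol item rolled at BeginPlay, then plays a death montage into ragdoll and timed removal.
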(event `self.ReceiveTick`
  (params (DeltaSeconds :type "Float (single-precision)"))
  (if (`self.Can_Move`)
    (bind _outactors (`GameplayStatics.GetAllActorsOfClass` "/Game/Blueprint/Character/BP_TopDownCharacter.BP_TopDownCharacter_C"))
    (bind _output (`|GetArrayItem` _outactors))
    (`/Engine/EditorBlueprintResources/StandardMacros.IsValid` _output
      (:`Is Valid`
        (`AIBlueprintHelperLibrary.SimpleMoveToActor` (`self.GetController`) _output)))))

(event `self.ReceiveBeginPlay`
  (set `self.Can_Move` true)
  (if (> (`KismetMathLibrary.RandomFloat`) (`self.Drop_Chance`))
    (bind _returnvalue (`|AddComponentByClass` "/Game/Blueprint/Actor_Component/BP_Drop_Item.BP_Drop_Item_C"))
    (set `self.Drop_Item` _returnvalue)))

(event `self.ReceiveAnyDamage`
  (params (Damage :type "Float (single-precision)") (DamageType :type "DamageType Object Reference") (InstigatedBy :type "Controller Object Reference") (DamageCauser :type "Actor Object Reference"))
  (if (not (`self.Is_Dead`))
    (`Health.Change_Health` (`self.Health`) Damage)))

(event `self.Health.On_Health_Change`
  (params (health :type "Float (single-precision)") (damage :type "Float (single-precision)"))
  (bind _returnvalue (`|SpawnActorFromClass` "/Game/Blueprint/Interaction_Environment/Display_Damage_Actor.Display_Damage_Actor_C" (`KismetMathLibrary.MakeTransform` (+ (`self.K2_GetActorLocation`) (`KismetMathLibrary.MakeVector` (`KismetMathLibrary.RandomFloatInRange` -10.0 10.0) (`KismetMathLibrary.RandomFloatInRange` -10.0 10.0)) (0.0 0.0 0.0))) "AlwaysSpawn" "MultiplyWithRoot" null null))
  (`/Game/Blueprint/Interaction_Environment/Display_Damage_Actor.Init_Actor` _returnvalue health damage)
  (if (> (`KismetMathLibrary.RandomFloat`) (`self.Stun_Chance`))
    (`self.Stun_On`)))

(event `self.Health.On_Dead`
  (bind _dead_animations (`self.Dead_Animations`))
  (bind _output (`|GetArrayItem` _dead_animations (- (`KismetArrayLibrary.Array_Length` _dead_animations) 1)))
  (set `self.Can_Move` false)
  (set `self.Can_Attack` false)
  (set `self.Is_Dead` true)
  (`|ExecutionSequence`
    (:`then_0`
      (`/Engine/EditorBlueprintResources/StandardMacros.IsValid` (`self.Drop_Item`)
        (:`Is Valid`
          (`/Game/Blueprint/Actor_Component/BP_Drop_Item.Drop` (`self.Drop_Item`) "Pistol"))))
    (:`then_1`
      (`/Engine/EditorBlueprintResources/StandardMacros.IsValid` _output
        (:`Is Valid`
          (`|PlayMontage` (`self.Mesh`) _output
            (:`OnCompleted`
              (`PrimitiveComponent.SetSimulatePhysics` (`self.Mesh`) true)
              (`PrimitiveComponent.SetCollisionProfileName` (`self.Mesh`) "PhysicsActor" true)
              (`self.SetLifeSpan` 5.0))
            (:`OnInterrupted`
              (`KismetSystemLibrary.PrintString` "Hello"))))
        (:`Is Not Valid`
          (`KismetSystemLibrary.PrintString` "Hello"))))))

(fn `Stun_Off`
  (set `self.Can_Move` true)
  (set `CharacterMovementComponent.MaxWalkSpeed` 400.0 (`self.CharacterMovement`)))

(fn `Stun_On`
  (set `self.Can_Move` false)
  (`KismetSystemLibrary.K2_SetTimer` null "Stun_Off" 2.8)
  (`self.PlayAnimMontage` "/Game/Blueprint/Enemy/Animations/zombie_scream_Montage.zombie_scream_Montage" 2.8)
  (set `CharacterMovementComponent.MaxWalkSpeed` 0.0 (`self.CharacterMovement`)))

(fn `UserConstructionScript`)