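; Base enemy, apparently a zombie, with health, a melee attack, random stuns and a chance to carry an item drop.
; Damage feeds the Health component, whose change event spawns a damage display and may trigger a timed stun.
; Attack montage notifies run a sphere trace that damages Player-tagged actors.
; Death drops the item, plays a montage, then ragdolls and expires; move/attack flags have getters, while the chase logic is unwired.
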(event `self.ReceiveBeginPlay`
  (set `self.Is_Can_Move` true)
  (if (> (`KismetMathLibrary.RandomFloat`) (`self.Chance_Drop`))
    (bind _returnvalue (`|AddComponentByClass` "/Game/Blueprint/Actor_Component/BP_Drop_Item.BP_Drop_Item_C"))
    (set `self.Drop_Item` _returnvalue)))

(event `self.ReceiveAnyDamage`
  (params (Damage :type "Float (single-precision)") (DamageType :type "DamageType Object Reference") (InstigatedBy :type "Controller Object Reference") (DamageCauser :type "Actor Object Reference"))
  (if (not (`self.Is_Dead`))
    (`Health.Change_Health` (`self.Health`) Damage)))

(event `self.Health.On_Health_Change`
  (params (health :type "Float (single-precision)") (damage :type "Float (single-precision)"))
  (bind _returnvalue (`|SpawnActorFromClass` "/Game/Blueprint/Interaction_Environment/Display_Damage_Actor.Display_Damage_Actor_C" (`KismetMathLibrary.MakeTransform` (+ (`self.K2_GetActorLocation`) (`KismetMathLibrary.MakeVector` (`KismetMathLibrary.RandomFloatInRange` -10.0 10.0) (`KismetMathLibrary.RandomFloatInRange` -10.0 10.0)) (0.0 0.0 0.0))) "AlwaysSpawn" "MultiplyWithRoot" null null))
  (`/Game/Blueprint/Interaction_Environment/Display_Damage_Actor.Init_Actor` _returnvalue health damage)
  (if (> (`KismetMathLibrary.RandomFloat`) (`self.Chance_Stun`))
    (`self.Stun_On`)))

(event `self.Health.On_Dead`
  (bind _anim_dead (`self.Anim_Dead`))
  (bind _output (`|GetArrayItem` _anim_dead (- (`KismetArrayLibrary.Array_Length` _anim_dead) 1)))
  (set `self.Is_Can_Move` false)
  (set `self.Is_Can_Attack` false)
  (set `self.Is_Dead` true)
  (`|ExecutionSequence`
    (:`then_0`
      (`/Engine/EditorBlueprintResources/StandardMacros.IsValid` (`self.Drop_Item`)
        (:`Is Valid`
          (`/Game/Blueprint/Actor_Component/BP_Drop_Item.Drop` (`self.Drop_Item`) "Pistol"))))
    (:`then_1`
      (`/Engine/EditorBlueprintResources/StandardMacros.IsValid` _output
        (:`Is Valid`
          (`|PlayMontage` (`self.Mesh`) _output
            (:`OnCompleted`
              (`PrimitiveComponent.SetSimulatePhysics` (`self.Mesh`) true)
              (`PrimitiveComponent.SetCollisionProfileName` (`self.Mesh`) "PhysicsActor" true)
              (`self.SetLifeSpan` 5.0))
            (:`OnInterrupted`
              (`KismetSystemLibrary.PrintString` "Hello"))))
        (:`Is Not Valid`
          (`KismetSystemLibrary.PrintString` "Hello"))))))

(event `/Game/Blueprint/Enemy/BPI_Combat.Attack`
  (bind _damage (`self.Damage`))
  (set `self.Is_Can_Attack` false)
  (set `self.Is_Can_Move` false)
  (bind _notifyname (`|PlayMontage` (`self.Mesh`) (`self.Anim_Attack`))
    (:`OnCompleted`
      (set `self.Is_Can_Attack` true :!label _label)
      (set `self.Is_Can_Move` true))
    (:`OnInterrupted`
      (goto _label))
    (:`OnNotifyBegin`
      (if (== _notifyname "Attack")
        (bind _outhit (`KismetSystemLibrary.SphereTraceSingle` (+ (`self.K2_GetActorLocation`) (* (`self.GetActorForwardVector`) 100.0)) (+ (`self.K2_GetActorLocation`) (* (`self.GetActorForwardVector`) 200.0)) (`self.Radius_Attack`) "TraceTypeQuery4" false (`|MakeArray` self :!type "Actor Object Reference") "ForDuration"))
        (bind (_bblockinghit _binitialoverlap _time _distance _location _impactpoint _normal _impactnormal _physmat _hitactor) (`GameplayStatics.BreakHitResult` _outhit))
        (`/Engine/EditorBlueprintResources/StandardMacros.IsValid` _hitactor
          (:`Is Valid`
            (if (`self.ActorHasTag` _hitactor "Player")
              (`GameplayStatics.ApplyDamage` _hitactor (`KismetMathLibrary.RandomFloatInRange` (+ _damage 5.0) (- _damage 5.0)) (`self.GetController`) self))))))))

(fn `Can_Attack`
  (returns (Can_Attack :type Boolean))
  (return (`self.Is_Can_Attack`)))

(fn `Can_Move`
  (returns (Can_Move :type Boolean))
  (return (`self.Is_Can_Move`)))

(fn `Stun_Off`
  (set `self.Is_Can_Move` true)
  (set `CharacterMovementComponent.MaxWalkSpeed` 400.0 (`self.CharacterMovement`)))

(fn `Stun_On`
  (set `self.Is_Can_Move` false)
  (`KismetSystemLibrary.K2_SetTimer` null "Stun_Off" 2.8)
  (`self.PlayAnimMontage` "/Game/Blueprint/Enemy/Animations/zombie_scream_Montage.zombie_scream_Montage" 2.8)
  (set `CharacterMovementComponent.MaxWalkSpeed` 0.0 (`self.CharacterMovement`)))

(fn `UserConstructionScript`)