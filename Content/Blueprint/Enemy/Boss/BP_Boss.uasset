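; Boss enemy with a melee attack and a projectile attack, exposing can-move and can-attack flags.
; Both attacks lock those flags, wait, then play a montage whose "Attack" notify fires a player-tagged sphere-trace hit or spawns a grenade-launcher projectile.
; Incoming damage feeds the Health component, which spawns damage display actors on change.
; On death it drops a pistol, plays a dying montage, then ragdolls before expiring.
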(event `self.Health.On_Dead`
  (set `self.Is_Can_Move` false)
  (set `self.Is_Can_Attack` false)
  (set `self.Is_Dead` true)
  (`|ExecutionSequence`
    (:`then_0`
      (`/Engine/EditorBlueprintResources/StandardMacros.IsValid` (`self.Drop_Item`)
        (:`Is Valid`
          (`/Game/Blueprint/Actor_Component/BP_Drop_Item.Drop` (`self.Drop_Item`) "Pistol"))))
    (:`then_1`
      (`|PlayMontage` (`self.Mesh`) "/Game/Blueprint/Enemy/Boss/Animations/Sequence/Mutant_Dying_Anim_Montage.Mutant_Dying_Anim_Montage"
        (:`OnCompleted`
          (`PrimitiveComponent.SetSimulatePhysics` (`self.Mesh`) true)
          (`PrimitiveComponent.SetCollisionProfileName` (`self.Mesh`) "PhysicsActor" true)
          (`self.SetLifeSpan` 5.0))
        (:`OnInterrupted`
          (`KismetSystemLibrary.PrintString` "Hello"))))))

(event `self.Health.On_Health_Change`
  (params (health :type "Float (single-precision)") (damage :type "Float (single-precision)"))
  (bind _returnvalue (`|SpawnActorFromClass` "/Game/Blueprint/Interaction_Environment/Display_Damage_Actor.Display_Damage_Actor_C" (`KismetMathLibrary.MakeTransform` (+ (`self.K2_GetActorLocation`) (`KismetMathLibrary.MakeVector` (`KismetMathLibrary.RandomFloatInRange` -10.0 10.0) (`KismetMathLibrary.RandomFloatInRange` -10.0 10.0)) (0.0 0.0 0.0))) "AlwaysSpawn" "MultiplyWithRoot" null null))
  (`/Game/Blueprint/Interaction_Environment/Display_Damage_Actor.Init_Actor` _returnvalue health damage))

(event `self.ReceiveAnyDamage`
  (params (Damage :type "Float (single-precision)") (DamageType :type "DamageType Object Reference") (InstigatedBy :type "Controller Object Reference") (DamageCauser :type "Actor Object Reference"))
  (if (not (`self.Is_Dead`))
    (`Health.Change_Health` (`self.Health`) Damage)))

(event `/Game/Blueprint/Enemy/Regular/BPI_Combat.Attack`
  (bind _damage (`self.Damage`))
  (set `self.Is_Can_Attack` false)
  (set `self.Is_Can_Move` false)
  (`KismetSystemLibrary.Delay` 1.0)
  (bind _notifyname (`|PlayMontage` (`self.Mesh`) (`self.Anim_Attack`))
    (:`OnCompleted`
      (set `self.Is_Can_Attack` true :!label _label)
      (set `self.Is_Can_Move` true))
    (:`OnInterrupted`
      (goto _label))
    (:`OnNotifyBegin`
      (if (== _notifyname "Attack")
        (bind _outhit (`KismetSystemLibrary.SphereTraceSingle` (+ (`self.K2_GetActorLocation`) (* (`self.GetActorForwardVector`) 100.0)) (+ (`self.K2_GetActorLocation`) (* (`self.GetActorForwardVector`) 200.0)) (`self.Radius_Attack`) "TraceTypeQuery4" false (`|MakeArray` self :!type "Actor Object Reference") "ForDuration"))
        (bind (_bblockinghit _binitialoverlap _time _distance _location _impactpoint _normal _impactnormal _physmat _hitactor) (`GameplayStatics.BreakHitResult` _outhit))
        (`/Engine/EditorBlueprintResources/StandardMacros.IsValid` _hitactor
          (:`Is Valid`
            (if (`self.ActorHasTag` _hitactor "Player")
              (`GameplayStatics.ApplyDamage` _hitactor (`KismetMathLibrary.RandomFloatInRange` (+ _damage 10.0) (- _damage 10.0)) (`self.GetController`) self))))))))

(event `/Game/Blueprint/Enemy/Regular/BPI_Combat.Boss_RPG_Attack`
  (set `self.Is_Can_Attack` false)
  (set `self.Is_Can_Move` false)
  (`KismetSystemLibrary.Delay` 1.0)
  (bind _notifyname (`|PlayMontage` (`self.Mesh`) (`self.Anim_Attack`))
    (:`OnCompleted`
      (set `self.Is_Can_Attack` true :!label _label_2)
      (set `self.Is_Can_Move` true))
    (:`OnInterrupted`
      (goto _label_2))
    (:`OnNotifyBegin`
      (if (== _notifyname "Attack")
        (bind _returnvalue (`|SpawnActorFromClass` "/Game/Items/Game_Actor/BP_Projectile_Grenade_Launcher.BP_Projectile_Grenade_Launcher_C" (`KismetMathLibrary.MakeTransform` (+ (`self.K2_GetActorLocation`) (0.0 300.0 0.0)) (`self.K2_GetActorRotation`)) "AlwaysSpawn" "MultiplyWithRoot" self null))
        (`Projectile_Default.Init` _returnvalue (make `Projectile_Info` "/Game/Blueprint/Enemy/Boss/BP_Projectile_RPG.BP_Projectile_RPG_C" "/Game/MilitaryWeapSilver/Weapons/GrenadeLauncherA_Ammo.GrenadeLauncherA_Ammo"))))))

(fn `Can_Attack`
  (returns (Can_Attack :type Boolean))
  (return (`self.Is_Can_Attack`)))

(fn `Can_Move`
  (returns (Can_Move :type Boolean))
  (return (`self.Is_Can_Move`)))

(fn `UserConstructionScript`)