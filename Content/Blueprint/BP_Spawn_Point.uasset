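; BP_Spawn_Point is a checkpoint that moves the player start when BP_TopDownCharacter overlaps its box.
; An inactive point deactivates every spawn point, then asks BP_Game_Mode for the player start using the "Checkpoint" name.
; It destroys that BP_Player_Start, spawns a replacement at its own transform and marks itself active.
; While active, it spins on roll every tick, independent of frame time.
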(event `self.Box.OnComponentBeginOverlap`
  (params (OverlappedComponent :type "PrimitiveComponent Object Reference") (OtherActor :type "Actor Object Reference") (OtherComp :type "PrimitiveComponent Object Reference") (OtherBodyIndex :type Integer) (bFromSweep :type Boolean) (SweepResult :type "HitResult Structure (by ref)"))
  (cast `/Game/Blueprint/Character/BP_TopDownCharacter` OtherActor
    (:`then`
      (if (not (`self.Is_Active`))
        ;[1 1 1] Need to change
        (bind _outactors (`GameplayStatics.GetAllActorsOfClass` "BP_Spawn_Point_C"))
        (for _array_element _outactors
          (set `/Game/Blueprint/BP_Spawn_Point.Is_Active` false _array_element))
        (bind _asbp_game_mode (cast `/Game/Blueprint/Game/Game/BP_Game_Mode` (`GameplayStatics.GetGameMode`))
          (:`then`
            (bind _asbp_player_start (cast `/Game/Blueprint/BP_Player_Start` (`GameModeBase.K2_FindPlayerStart` _asbp_game_mode (`GameplayStatics.GetPlayerController` 0) "Checkpoint"))
              (:`then`
                (`self.K2_DestroyActor` _asbp_player_start)
                (`|SpawnActorFromClass` "/Game/Blueprint/BP_Player_Start.BP_Player_Start_C" (`self.GetTransform`) "AlwaysSpawn" "MultiplyWithRoot" null null)
                (set `self.Is_Active` true))
              (:`CastFailed`
                (`KismetSystemLibrary.PrintString` "Hello"))))
          (:`CastFailed`
            (`KismetSystemLibrary.PrintString` "Hello")))))
    (:`CastFailed`
      (`KismetSystemLibrary.PrintString` (`KismetSystemLibrary.GetDisplayName` OtherActor)))))

(event `self.ReceiveTick`
  (params (DeltaSeconds :type "Float (single-precision)"))
  (bind _returnvalue_roll (`KismetMathLibrary.BreakRotator` (`self.K2_GetActorRotation`)))
  (if (`self.Is_Active`)
    (`self.K2_SetActorRotation` (`KismetMathLibrary.MakeRotator` (+ _returnvalue_roll 5.0)))))

(fn `UserConstructionScript`)