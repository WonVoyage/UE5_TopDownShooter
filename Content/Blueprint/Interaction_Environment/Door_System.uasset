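; Door Blueprint that slides open and closed vertically as the top-down player character passes through its trigger volumes.
; Overlapping Trigger_Enter calls Opening and overlapping Trigger_Exit calls Closing, both responding only to BP_TopDownCharacter.
; A DoorOpen flag blocks repeat calls, while the Opening_Door timeline drives the door's relative Z offset, playing forward to open and in reverse to close.
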(event `self.Trigger_Enter.OnComponentBeginOverlap`
  (params (OverlappedComponent :type "PrimitiveComponent Object Reference") (OtherActor :type "Actor Object Reference") (OtherComp :type "PrimitiveComponent Object Reference") (OtherBodyIndex :type Integer) (bFromSweep :type Boolean) (SweepResult :type "HitResult Structure (by ref)"))
  (cast `/Game/Blueprint/Character/BP_TopDownCharacter` OtherActor)
  (`self.Opening`))

(event `self.Trigger_Exit.OnComponentBeginOverlap`
  (params (OverlappedComponent :type "PrimitiveComponent Object Reference") (OtherActor :type "Actor Object Reference") (OtherComp :type "PrimitiveComponent Object Reference") (OtherBodyIndex :type Integer) (bFromSweep :type Boolean) (SweepResult :type "HitResult Structure (by ref)"))
  (cast `/Game/Blueprint/Character/BP_TopDownCharacter` OtherActor)
  (`self.Closing`))

(event `Opening`
  (if (not (`self.Door_Open`))
    (set `self.Door_Open` true)
    (bind (_direction _offset_z) (`Timeline|Opening_Door` :!via `PlayFromStart` :!label _label)
      (:`Update`
        (`SceneComponent.K2_SetRelativeLocation` (`self.Door`) (`KismetMathLibrary.MakeVector` 0.0 0.0 _offset_z) false false)))))

(event `Closing`
  (if (`self.Door_Open`)
    (set `self.Door_Open` false)
    (goto _label :!via `ReverseFromEnd`)))

(fn `UserConstructionScript`)