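; Ammo pickup actor that adds ammunition to a character's inventory on overlap.
; It extends a parent pickup, overriding the character overlap event to ask the inventory whether it can take ammo for the pickup's weapon type.
; If allowed, it adds its count to that weapon's ammo slot; otherwise it prints a debug message.
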(event `self.Overlap_Character`
  (params (Inventory :type "Inventory Object Reference"))
  (bind _output_get (set `self.Inventory_0` Inventory))
  (`parent.Overlap_Character` _output_get)
  (bind _returnvalue (`Inventory.Can_Pickup_Ammo` (`self.Inventory_0`) (`self.Weapon_Type`)))
  (if _returnvalue
    (`Inventory.Ammo_Slot_Change_Value` (`self.Inventory_0`) (`self.Weapon_Type`) (`self.Count`))
    (else
      (`KismetSystemLibrary.PrintString` "I can't pickup!!!"))))

(fn `UserConstructionScript`
  (`parent.UserConstructionScript`))