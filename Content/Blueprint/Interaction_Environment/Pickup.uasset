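; Base world pickup actor that hands an overlapping top-down character's inventory to an overlap event, left empty here.
; A sphere overlap casts to BP_TopDownCharacter and passes its Inventory to that event; PickupSuccess destroys the actor.
; InitActor shows the item's static mesh, or its skeletal mesh as fallback, destroying the unused component.
; DropItem spawns a new Pickup at this actor's location and initializes it with the given item.
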(event `Overlap_Character`
  (params (Inventory :type "Inventory Object Reference")))

(event `self.Sphere.OnComponentBeginOverlap`
  (params (OverlappedComponent :type "PrimitiveComponent Object Reference") (OtherActor :type "Actor Object Reference") (OtherComp :type "PrimitiveComponent Object Reference") (OtherBodyIndex :type Integer) (bFromSweep :type Boolean) (SweepResult :type "HitResult Structure (by ref)"))
  (bind _asbp_top_down_character (cast `/Game/Blueprint/Character/BP_TopDownCharacter` OtherActor))
  (bind _output_get (set `self.Inventory` (`TDSCharacter.Inventory` _asbp_top_down_character)))
  (`self.Overlap_Character` _output_get))

(fn `Drop_Item`
  (params (Item :type "Drop_Item Structure"))
  (bind _returnvalue (`|SpawnActorFromClass` "Pickup_C" (`KismetMathLibrary.MakeTransform` (`self.K2_GetActorLocation`)) "Undefined" "MultiplyWithRoot" null null))
  (`self.Init_Actor` :`self` _returnvalue :`Item` Item))

(fn `Init_Actor`
  (params (Item :type "Drop_Item Structure") (Info :type "Weapon_Info Structure"))
  (bind (_static_mesh _skeletal_mesh) (break `Drop_Item` Item))
  (`/Engine/EditorBlueprintResources/StandardMacros.IsValid` _static_mesh
    (:`Is Valid`
      (`ActorComponent.K2_DestroyComponent` (`self.SkeletalMesh`))
      (`StaticMeshComponent.SetStaticMesh` (`self.StaticMesh`) _static_mesh))
    (:`Is Not Valid`
      (`/Engine/EditorBlueprintResources/StandardMacros.IsValid` _skeletal_mesh
        (:`Is Valid`
          (`ActorComponent.K2_DestroyComponent` (`self.StaticMesh`))
          (`SkeletalMeshComponent.SetSkeletalMeshAsset` (`self.SkeletalMesh`) _skeletal_mesh))
        (:`Is Not Valid`
          (`KismetSystemLibrary.PrintString` "Error Drop Item Not Have Any Mesh"))))))

(fn `Pickup_Success`
  (`self.K2_DestroyActor`))

(fn `UserConstructionScript`)