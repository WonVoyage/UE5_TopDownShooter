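; Destructible environment actor that takes damage through a Health component and is destroyed when that health runs out.
; AnyDamage prints the amount and passes it to Health, whose change event spawns a Display_Damage_Actor at a randomly jittered offset to show health and damage.
; On death it waits a tiny delay before destroying itself.
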(event `self.Health.On_Dead`
  (`KismetSystemLibrary.Delay` 0.0001)
  (`self.K2_DestroyActor`))

(event `self.ReceiveAnyDamage`
  (params (Damage :type "Float (single-precision)") (DamageType :type "DamageType Object Reference") (InstigatedBy :type "Controller Object Reference") (DamageCauser :type "Actor Object Reference"))
  (`KismetSystemLibrary.PrintString` (`KismetStringLibrary.Conv_DoubleToString` Damage))
  (`Health.Change_Health` (`self.Health`) Damage))

(event `self.Health.On_Health_Change`
  (params (health :type "Float (single-precision)") (damage :type "Float (single-precision)"))
  (bind _returnvalue (`|SpawnActorFromClass` "/Game/Blueprint/Interaction_Environment/Display_Damage_Actor.Display_Damage_Actor_C" (`KismetMathLibrary.MakeTransform` (+ (`self.K2_GetActorLocation`) (`KismetMathLibrary.MakeVector` (`KismetMathLibrary.RandomFloatInRange` -10.0 10.0) (`KismetMathLibrary.RandomFloatInRange` -10.0 10.0)) (`self.Health_Number_Local_Spawn_Point`))) "AlwaysSpawn" "MultiplyWithRoot" null null))
  (`/Game/Blueprint/Interaction_Environment/Display_Damage_Actor.Init_Actor` _returnvalue health damage))

(fn `UserConstructionScript`)