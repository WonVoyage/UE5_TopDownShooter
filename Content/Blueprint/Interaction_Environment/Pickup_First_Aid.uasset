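; First aid pickup that heals the top-down player character when overlapped.
; It extends a parent pickup's OverlapCharacter event, casting the inventory's owner to BP_TopDownCharacter and reading its Health component.
; Only below 100 health does it apply its Value as a health change and call PickupSuccess, so it is not used at full health.
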(event `self.Overlap_Character`
  (params (Inventory :type "Inventory Object Reference"))
  (`parent.Overlap_Character` Inventory)
  (bind _asbp_top_down_character (cast `/Game/Blueprint/Character/BP_TopDownCharacter` (`ActorComponent.GetOwner` Inventory)))
  (bind _health (`TDSCharacter.Health` _asbp_top_down_character))
  (bind _returnvalue (`Health.Get_Current_Health` _health))
  (if (< _returnvalue 100.0)
    (`Health.Change_Health` _health (`self.value`))
    (`self.Pickup_Success`)))

(fn `UserConstructionScript`
  (`parent.UserConstructionScript`))