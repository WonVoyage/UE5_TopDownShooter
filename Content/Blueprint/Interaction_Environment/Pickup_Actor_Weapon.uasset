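; Weapon pickup actor that gives a weapon to a character's inventory on overlap, built on a parent pickup class.
; The overlap override runs the parent logic, passes its NewWeapon to the inventory's GetWeaponToInventory, and calls PickupSuccess only when that returns true.
; InitActor copies the slot from the supplied item before running the parent's initialization.
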(event `self.Overlap_Character`
  (params (Inventory :type "Inventory Object Reference"))
  (`parent.Overlap_Character` Inventory)
  (bind _returnvalue (`Inventory.Get_Weapon_To_Inventory` Inventory (`self.New_Weapon`)))
  (if _returnvalue
    (`self.Pickup_Success`)))

(fn `Init_Actor`
  (params (Item :type "Drop_Item Structure"))
  (set `self.Slot` (`.Slot` (break `Drop_Item` Item)))
  (`parent.Init_Actor` Item))

(fn `UserConstructionScript`
  (`parent.UserConstructionScript`))